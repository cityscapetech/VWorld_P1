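; Hologram actor that spins slowly about its vertical axis every tick and lets the player turn and zoom it.
; It enables input from player 0 on BeginPlay, and the RotateObjectX axis yaws the Cube.
; Right and left mouse presses lengthen and shorten the SpringArm in fixed steps, opposite to their Zoom In/Out labels.
; Cube scale-up and scale-down nodes exist but are not connected to any event.
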(event EventTick
  (params (DeltaSeconds :type Float%20%28single-precision%29))
  (Class|Actor|AddActorWorldRotation (Math|Rotator|MakeRotator 0.0 0.0 0.8)))

(event EventBeginPlay
  ;[1 1 1] Input Enable
  (Input|EnableInput (Game|GetPlayerController 0)))

(event Input|AxisEvents|InputAxisRotateObjectX
  (params (AxisValue :type Float%20%28single-precision%29))
  ;[1 1 1] Panning
  (Transformation|AddWorldRotation (Variables|Default|GetCube) (Math|Rotator|MakeRotator 0.0 0.0 (* AxisValue -1.0)) false false))

(event Input|MouseEvents|LeftMouseButton
  (params (Key :type Key%20Structure))
  ;[1 1 1] Scale Down
)

(event Input|MouseEvents|RightMouseButton
  (params (Key :type Key%20Structure))
  ;[1 1 1] Scale Up
)

(event Input|MouseEvents|LeftMouseButton
  (params (Key :type Key%20Structure))
  ;[1 1 1] Zoom out
  (:Pressed
    (Variables|/Script/Engine.SpringArmComponent|SetTargetArmLength (Variables|Default|GetSpringArm) (- (Variables|/Script/Engine.SpringArmComponent|GetTargetArmLength (Variables|Default|GetSpringArm)) 5e+01))))

(event Input|MouseEvents|RightMouseButton
  (params (Key :type Key%20Structure))
  ;[1 1 1] Zoom In
  (:Pressed
    (Variables|/Script/Engine.SpringArmComponent|SetTargetArmLength (Variables|Default|GetSpringArm) (+ 5e+01 (Variables|/Script/Engine.SpringArmComponent|GetTargetArmLength (Variables|Default|GetSpringArm))))))

(fn ConstructionScript)