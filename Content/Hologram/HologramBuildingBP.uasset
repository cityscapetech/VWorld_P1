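; Hologram building actor that the player can rotate and zoom the view on.
; BeginPlay enables input from player 0, and the RotateObjectX axis yaws the Cone component in world space, inverted.
; The mouse wheel lengthens (down) or shortens (up) the SpringArm in fixed steps, with no clamping.
; Scaling, constant spin and IsPossessed logic are left disconnected and never run.
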(event EventTick
  (params (DeltaSeconds :type Float%20%28single-precision%29)))

(event EventBeginPlay
  ;[1 1 1] Input Enable
  (Input|EnableInput (Game|GetPlayerController 0)))

(event Input|AxisEvents|InputAxisRotateObjectX
  (params (AxisValue :type Float%20%28single-precision%29))
  ;[1 1 1] Panning
  (Transformation|AddWorldRotation (Variables|Default|GetCone) (Math|Rotator|MakeRotator 0.0 0.0 (* AxisValue -1.0)) false false))

(event Input|KeyboardEvents|1
  (params (Key :type Key%20Structure :default "None")))

(event Input|MouseEvents|MouseWheelDown
  (params (Key :type Key%20Structure :default "None"))
  ;[1 1 1] Zoom In
  (:Pressed
    (Variables|/Script/Engine.SpringArmComponent|SetTargetArmLength (Variables|Default|GetSpringArm) (+ 5e+01 (Variables|/Script/Engine.SpringArmComponent|GetTargetArmLength (Variables|Default|GetSpringArm))))))

(event Input|MouseEvents|MouseWheelUp
  (params (Key :type Key%20Structure :default "None"))
  ;[1 1 1] Zoom out
  (:Pressed
    (Variables|/Script/Engine.SpringArmComponent|SetTargetArmLength (Variables|Default|GetSpringArm) (- (Variables|/Script/Engine.SpringArmComponent|GetTargetArmLength (Variables|Default|GetSpringArm)) 5e+01))))

(event Input|MouseEvents|MouseWheelDown
  (params (Key :type Key%20Structure :default "None"))
  ;[1 1 1] Scale Up
)

(event Input|MouseEvents|MouseWheelUp
  (params (Key :type Key%20Structure :default "None"))
  ;[1 1 1] Scale Down
)

(fn ConstructionScript)