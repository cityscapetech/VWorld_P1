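; Meeting controller actor that stages a virtual-world meeting: agent arrival, seated avatars and listings screen.
; On first BeginPlay it caches the player character, then runs a timed Niagara spawn-in for the player's MetaHuman and the Madeeha agent.
; Key 1 or FadeInAndSit fades the camera, shows all SkeletalMeshActors as sitters and hides third-person character meshes.
; ShowListingsUI replaces any web browser actor with BP_Listings at a fixed location.
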(event Custom|SpawnAgent
  (bind _returnvalue (Transformation|GetActorTransform))
  ;[1 1 1] AGENT SPAWNING
  (Variables|/Script/Engine.PlayerController|SetbShowMouseCursor (Game|GetPlayerController 0) true)
  (bind _asbp_abdullah_metahuman_v_5 (Utilities|Casting|CastToBP_Abdullah_Metahuman_v5 (Variables|Default|GetThirdPersonBP_Ref)))
  (Default|SetVisibilityMH _asbp_abdullah_metahuman_v_5 false)
  (Niagara|SpawnSystematLocation "/Game/Assets/SpawnFX/SpawnEffect.SpawnEffect" (- (Transformation|GetActorLocation (Variables|Default|GetThirdPersonBP_Ref)) "0.000000,0.000000,92.000000"))
  (Utilities|FlowControl|Delay 2.25)
  (bind _asbp_abdullah_metahuman_v_5_2 (Utilities|Casting|CastToBP_Abdullah_Metahuman_v5 (Variables|Default|GetThirdPersonBP_Ref)))
  (Default|SetVisibilityMH _asbp_abdullah_metahuman_v_5_2 true)
  (Utilities|FlowControl|Delay 2.0)
  (Niagara|SpawnSystematLocation "/Game/Assets/SpawnFX/SpawnEffect.SpawnEffect" (.location _returnvalue) (.rotation _returnvalue))
  (Utilities|FlowControl|Delay 2.0)
  (Game|SpawnActorfromClass "/Game/MetaHumans/Madeeha_MH_v2/BP_Madeeha_MH_v2.BP_Madeeha_MH_v2_C" (Math|Transform|MakeTransform (+ (.location (Transformation|GetActorTransform)) "0.000000,0.000000,100.000000") "0.000000,180.000000,0.000000" "1.000000,1.000000,1.000000") "Undefined" 0 0))

(event Custom|HideSittingAvatars
  ;[1 1 1] HIDE SITTING AVATARS
  (bind _outactors (Actor|GetAllActorsOfClass "/Script/Engine.SkeletalMeshActor"))
  (for _array_element _outactors
    (Rendering|SetVisibility (Variables|/Script/Engine.SkeletalMeshActor|GetSkeletalMeshComponent _array_element) false false)))

(event Custom|Set%20Third%20Person%20Reference
  ;[1 1 1] THIRDPERSON CHARACTER REFERENCE
  (bind _asbp_third_person_character (Utilities|Casting|CastToBP_ThirdPersonCharacter (Game|GetPlayerCharacter 0)))
  (Variables|Default|SetThirdPersonBP_Ref _asbp_third_person_character)
  (Input|EnableInput (Game|GetPlayerController 0)))

(event Custom|ShowSittingAvatars
  ;[1 1 1] SHOW SITTING AVATARS
  (bind _outactors (Actor|GetAllActorsOfClass "/Script/Engine.SkeletalMeshActor"))
  (for _array_element _outactors
    (Rendering|SetVisibility (Variables|/Script/Engine.SkeletalMeshActor|GetSkeletalMeshComponent _array_element) true false)))

(event Custom|FadeInAndSit
  ;[1 1 1] CAMERA FADE
  (CameraFades|StartCameraFade :self (Game|GetPlayerCameraManager 0) :ToAlpha 1.0 :Duration 1.0 :bHoldWhenFinished true)
  (Utilities|FlowControl|Delay 2.0)
  (CallFunction|ShowSittingAvatars)
  (bind _outactors (Actor|GetAllActorsOfClass "/Game/Assets/ThirdPerson/Blueprints/BP_ThirdPersonCharacter.BP_ThirdPersonCharacter_C"))
  (for _array_element _outactors
    (Rendering|SetVisibility (Variables|/Script/Engine.Character|GetMesh _array_element) false false)
    (CameraFades|StartCameraFade :self (Game|GetPlayerCameraManager 0) :FromAlpha 1.0 :Duration 1.0 :bHoldWhenFinished true)
    (if (not (Variables|Default|GetfirstTime))
      (Input|DisableInput (Variables|Default|GetThirdPersonBP_Ref) (Game|GetPlayerController 0))
      (Development|PrintString "Sitting" true true "(R=0.000000,G=0.357935,B=1.000000,A=1.000000)" 2e+01))))

(event Custom|ShowListingsUI
  (bind _returnvalue (Actor|GetActorOfClass "/Game/VirtualWorld/InGameBrowser/Blueprints/BP_WebBrowser.BP_WebBrowser_C"))
  (Utilities|IsValid _returnvalue
    (:Is%20Valid
      (Actor|DestroyActor _returnvalue)
      (Game|SpawnActorfromClass "/Game/VirtualWorld/InGameBrowser/Blueprints/BP_Listings.BP_Listings_C" (Math|Transform|MakeTransform "-295.000000,4452.000000,380.000000" "0, 0, 0" "1.000000,1.000000,1.000000") "Undefined" 0 0))
    (:Is%20Not%20Valid
      (Game|SpawnActorfromClass "/Game/VirtualWorld/InGameBrowser/Blueprints/BP_Listings.BP_Listings_C" (Math|Transform|MakeTransform "-295.000000,4452.000000,380.000000" "0, 0, 0" "1.000000,1.000000,1.000000") "Undefined" 0 0))))

(event Custom|ActivateSittingAvatars
  ;[1 1 1] CAMERA FADE
  (CameraFades|StartCameraFade :self (Game|GetPlayerCameraManager 0) :ToAlpha 1.0 :Duration 1.0 :bHoldWhenFinished true)
  (Utilities|FlowControl|Delay 2.0)
  (CallFunction|ShowSittingAvatars)
  (bind _outactors (Actor|GetAllActorsOfClass "/Game/Assets/ThirdPerson/Blueprints/BP_ThirdPersonCharacter.BP_ThirdPersonCharacter_C"))
  (for _array_element _outactors
    (Rendering|SetVisibility (Variables|/Script/Engine.Character|GetMesh _array_element) false false)
    (CameraFades|StartCameraFade :self (Game|GetPlayerCameraManager 0) :FromAlpha 1.0 :Duration 1.0 :bHoldWhenFinished true)
    (if (not (Variables|Default|GetfirstTime))
      (Input|DisableInput (Variables|Default|GetThirdPersonBP_Ref) (Game|GetPlayerController 0))
      (Development|PrintString "Sitting" true true "(R=0.000000,G=0.357935,B=1.000000,A=1.000000)" 2e+01))))

(event EventBeginPlay
  (if (not (Variables|Default|GetfirstTime))
    (Variables|Default|SetfirstTime true)
    (CallFunction|SetThirdPersonReference)
    (CallFunction|SpawnAgent)))

(event Input|KeyboardEvents|1
  (params (Key :type Key%20Structure :default "None"))
  (:Pressed
    (CallFunction|ActivateSittingAvatars)))

(fn ConstructionScript)