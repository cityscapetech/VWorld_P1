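; Trigger actor that shows the home office interior subtitle and plays its audio in the virtual world.
; When its Box component is first overlapped, a Once flag blocks repeat triggers, the W_InteriorST_HomeOffice widget is added to the viewport, and the Home_Office sound plays at the actor's location.
; After fixed delays it removes the widget and destroys itself, making it a one-shot trigger.
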(event OnComponentBeginOverlap(Box)
  (params (OverlappedComponent :type Primitive%20Component%20Object%20Reference) (OtherActor :type Actor%20Object%20Reference) (OtherComp :type Primitive%20Component%20Object%20Reference) (OtherBodyIndex :type Integer) (bFromSweep :type Boolean) (SweepResult :type Hit%20Result%20Structure%20%28by%20ref%29))
  (if (not (Variables|Default|Getonce))
    (Variables|Default|Setonce true)
    (bind _returnvalue (UserInterface|CreateWidget "/Game/VirtualWorld/Widgets/Interior_Subtitles/W_InteriorST_HomeOffice.W_InteriorST_HomeOffice_C"))
    (UserInterface|Viewport|AddtoViewport _returnvalue 0)
    (Audio|PlaySoundatLocation "/Game/SubtitleSystem/SoundClips/InteriorPresets/Home_Office.Home_Office" (Transformation|GetActorLocation) "0, 0, 0" 1.0 1.0 0.0 0 0 0 0)
    (Utilities|FlowControl|Delay 6.0)
    (Widget|RemovefromParent _returnvalue)
    (Utilities|FlowControl|Delay 0.2)
    (Actor|DestroyActor)))

(event EventBeginPlay)

(event Collision|EventActorBeginOverlap
  (params (OtherActor :type Actor%20Object%20Reference)))

(event EventTick
  (params (DeltaSeconds :type Float%20%28single-precision%29)))

(fn ConstructionScript)