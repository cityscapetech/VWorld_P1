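; Actor that plays a radius-based outline post-process transition for virtual-world level changes.
; Both events weight the blue outline material over the black one on the player's follow camera, then timelines animate Radius in PC_Outline.
; The reverse transition also centers the effect on the actor and, when finished, streams in InteriorPreset2 and unloads MeetingRoom2.
; BlackFirst is an empty stub with disconnected weight-swap nodes.
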(event Custom|TransitionFromReverse
  (CallFunction|BlueFirst)
  (Rendering|Material|SetVectorParameterValue "/Game/Materials/PC_Outline.PC_Outline" "Position" (Math|Conversions|ToLinearColor(Vector) (Transformation|GetWorldLocation (Variables|Default|GetDefaultSceneRoot))) :!class /Script/Engine.KismetMaterialLibrary)
  (bind _newtrack_0 (Timeline|Timeline ReverseFromEnd)
    (:Update
      (Rendering|Material|SetScalarParameterValue "/Game/Materials/PC_Outline.PC_Outline" "Radius" _newtrack_0 :!class /Script/Engine.KismetMaterialLibrary))
    (:Finished
      (Game|LoadStreamLevel(byName) "InteriorPreset2" true)
      (Game|UnloadStreamLevel(byName) "MeetingRoom2" false))))

(event Custom|TransitionFromStart
  (CallFunction|BlueFirst)
  (bind _newtrack_0 (Timeline|Timeline_0 PlayFromStart)
    (:Update
      (Rendering|Material|SetScalarParameterValue "/Game/Materials/PC_Outline.PC_Outline" "Radius" _newtrack_0 :!class /Script/Engine.KismetMaterialLibrary))))

(fn ConstructionScript)

(fn BlueFirst
  (bind _asbp_third_person_character (Utilities|Casting|CastToBP_ThirdPersonCharacter (Game|GetPlayerCharacter 0)))
  (Utilities|Array|SetArrayElem (.array (Utilities|Struct|BreakPostProcessSettings (Variables|/Script/Engine.CameraComponent|GetPostProcessSettings (Variables|/Game/Assets/ThirdPerson/Blueprints/BP_ThirdPersonCharacter.BP_ThirdPersonCharacter_C|GetFollowCamera _asbp_third_person_character)))) 0 (Utilities|Struct|MakeWeightedBlendable 1.0 "/Game/Materials/PM_Outlines_Inst.PM_Outlines_Inst"))
  (Utilities|Array|SetArrayElem (.array (Utilities|Struct|BreakPostProcessSettings (Variables|/Script/Engine.CameraComponent|GetPostProcessSettings (Variables|/Game/Assets/ThirdPerson/Blueprints/BP_ThirdPersonCharacter.BP_ThirdPersonCharacter_C|GetFollowCamera _asbp_third_person_character)))) 1 (Utilities|Struct|MakeWeightedBlendable 0.0 "/Game/Materials/PM_Outlines_BlackInst.PM_Outlines_BlackInst")))

(fn BlackFirst)