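; Subtitle manager that shows narration lines onscreen and plays their matching 2D sound.
; On BeginPlay it creates a W_Subtitles widget, adds it to the viewport and blanks it.
; ShowLine forwards a narration DataTable to ShowNextLine, which displays the current row's text, plays its sound and increments the row index.
; Each call advances one line, with FirstLine restarting at the top; nothing here auto-advances or clears after playback.
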(event Custom|ClearSubtitles
  ;[1 1 1] Clear Subtitle line
  (Default|DisplayLine (Variables|Default|GetSubtitlesWidgetReference)))

(event Custom|ShowNextLine
  (params (NarrationList :type Data%20Table%20Object%20Reference) (FirstLine :type Boolean))
  ;[1 1 1] Get next line to display
  (Variables|Default|SetNarration%20List NarrationList)
  (if FirstLine
    ;[1 1 1] After checking if first line, gets required data
    (Variables|Default|SetCurrentRow 0))
  (bind _outrownames (DataTable|GetDataTableRowNames (Variables|Default|GetNarration%20List)))
  (bind _returnvalue (Utilities|GetDataTableRow (Variables|Default|GetNarration%20List) (Utilities|Array|Get(acopy) _outrownames (Variables|Default|GetCurrentRow)))
    (:then
      (Default|DisplayLine (Variables|Default|GetSubtitlesWidgetReference) (.LineToShow (Utilities|Struct|BreakStruct_Subtitles _returnvalue)))
      (Audio|PlaySound2D (.NarrationSound (Utilities|Struct|BreakStruct_Subtitles _returnvalue)) 1.0 1.0 0.0 0 0)
      (Math|Integer|IncrementInt (Variables|Default|GetCurrentRow)))))

(event EventBeginPlay
  ;[1 1 1] Display Subtitles onscreen via Widget
  (bind _returnvalue (UserInterface|CreateWidget "/Game/SubtitleSystem/W_Subtitles.W_Subtitles_C"))
  (bind _output_get (Variables|Default|SetSubtitlesWidgetReference _returnvalue))
  (UserInterface|Viewport|AddtoViewport _output_get 0)
  (CallFunction|ClearSubtitles))

(fn ConstructionScript)

(fn ShowLine
  (params (NarrationList :type Data%20Table%20Object%20Reference) (FirstLine :type Boolean))
  (CallFunction|ShowNextLine NarrationList FirstLine))