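; Meeting controller actor that stages a virtual-world meeting with a spawned agent, seated avatars and a swappable display.
; BeginPlay hides all SkeletalMeshActors, then plays timed spawn effects to reveal the player and spawn a re-skinned third-person character as the agent.
; Key 1 or FadeInAndSit fakes sitting through a camera fade, swapping characters for seated avatars and disabling player input.
; Keys 2 and 3 swap BP_Listings and BP_WebBrowser at a fixed location; ShowListingsUI also triggers listings.
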(event Custom|SpawnAgent
  (bind _returnvalue (Transformation|GetActorTransform))
  (bind _returnvalue_2 (Transformation|GetActorTransform))
  ;[1 1 1] AGENT SPAWNING
  (Variables|/Script/Engine.PlayerController|SetbShowMouseCursor (Game|GetPlayerController 0) true)
  (Rendering|SetVisibility (Variables|/Script/Engine.Character|GetMesh (Variables|Default|GetThirdPersonBP_Ref)) false false)
  (Niagara|SpawnSystematLocation "/Game/Assets/SpawnFX/SpawnEffect.SpawnEffect" (- (Transformation|GetActorLocation (Variables|Default|GetThirdPersonBP_Ref)) "0.000000,0.000000,92.000000"))
  (Utilities|FlowControl|Delay 2.25)
  (Rendering|SetVisibility (Variables|/Script/Engine.Character|GetMesh (Variables|Default|GetThirdPersonBP_Ref)) true false)
  (Utilities|FlowControl|Delay 2.0)
  (Niagara|SpawnSystematLocation "/Game/Assets/SpawnFX/SpawnEffect.SpawnEffect" (.location _returnvalue_2) (.rotation _returnvalue_2))
  (Utilities|FlowControl|Delay 2.0)
  (bind _returnvalue_3 (Game|SpawnActorfromClass "/Game/Assets/ThirdPerson/Blueprints/BP_ThirdPersonCharacter.BP_ThirdPersonCharacter_C" (Math|Transform|MakeTransform (+ (.location _returnvalue) "0.000000,0.000000,100.000000") (.rotation _returnvalue) "1.000000,1.000000,1.000000") "Undefined" 0 0))
  (Rendering|Material|SetMaterial (Variables|/Script/Engine.Character|GetMesh _returnvalue_3) 0 "/Game/Assets/Characters/Mannequins/Materials/Instances/Manny/MI_Manny_02.MI_Manny_02")
  (Rendering|Material|SetMaterial (Variables|/Script/Engine.Character|GetMesh _returnvalue_3) 1 "/Game/Assets/Characters/Mannequins/Materials/Instances/Manny/MI_Manny_01.MI_Manny_01"))

(event Custom|HideSittingAvatars
  ;[1 1 1] HIDE SITTING AVATARS
  (bind _outactors (Actor|GetAllActorsOfClass "/Script/Engine.SkeletalMeshActor"))
  (for _array_element _outactors
    (Rendering|SetVisibility (Variables|/Script/Engine.SkeletalMeshActor|GetSkeletalMeshComponent _array_element) false false)))

(event Custom|Set%20Third%20Person%20Reference
  ;[1 1 1] THIRDPERSON CHARACTER REFERENCE
  (bind _asbp_third_person_character (Utilities|Casting|CastToBP_ThirdPersonCharacter (Game|GetPlayerCharacter 0)))
  (Variables|Default|SetThirdPersonBP_Ref _asbp_third_person_character)
  (Input|EnableInput (Game|GetPlayerController 0)))

(event Custom|ShowSittingAvatars
  ;[1 1 1] SHOW SITTING AVATARS
  (bind _outactors (Actor|GetAllActorsOfClass "/Script/Engine.SkeletalMeshActor"))
  (for _array_element _outactors
    (Rendering|SetVisibility (Variables|/Script/Engine.SkeletalMeshActor|GetSkeletalMeshComponent _array_element) true false)))

(event Custom|FadeInAndSit
  ;[1 1 1] CAMERA FADE
  (CameraFades|StartCameraFade :self (Game|GetPlayerCameraManager 0) :ToAlpha 1.0 :Duration 1.0 :bHoldWhenFinished true)
  (Utilities|FlowControl|Delay 2.0)
  (CallFunction|ShowSittingAvatars)
  (bind _outactors (Actor|GetAllActorsOfClass "/Game/Assets/ThirdPerson/Blueprints/BP_ThirdPersonCharacter.BP_ThirdPersonCharacter_C"))
  (for _array_element _outactors
    (Rendering|SetVisibility (Variables|/Script/Engine.Character|GetMesh _array_element) false false)
    (CameraFades|StartCameraFade :self (Game|GetPlayerCameraManager 0) :FromAlpha 1.0 :Duration 1.0 :bHoldWhenFinished true)
    (Input|DisableInput (Variables|Default|GetThirdPersonBP_Ref) (Game|GetPlayerController 0))))

(event Custom|ShowListingsUI
  (bind _returnvalue (Actor|GetActorOfClass "/Game/VirtualWorld/InGameBrowser/Blueprints/BP_WebBrowser.BP_WebBrowser_C"))
  (Utilities|IsValid _returnvalue
    (:Is%20Valid
      (Actor|DestroyActor _returnvalue)
      (Game|SpawnActorfromClass "/Game/VirtualWorld/InGameBrowser/Blueprints/BP_Listings.BP_Listings_C" (Math|Transform|MakeTransform "-295.000000,4452.000000,380.000000" "0, 0, 0" "1.000000,1.000000,1.000000") "Undefined" 0 0))
    (:Is%20Not%20Valid
      (Game|SpawnActorfromClass "/Game/VirtualWorld/InGameBrowser/Blueprints/BP_Listings.BP_Listings_C" (Math|Transform|MakeTransform "-295.000000,4452.000000,380.000000" "0, 0, 0" "1.000000,1.000000,1.000000") "Undefined" 0 0))))

(event EventBeginPlay
  (CallFunction|SetThirdPersonReference)
  (CallFunction|SpawnAgent)
  (CallFunction|HideSittingAvatars))

(event Input|KeyboardEvents|1
  (params (Key :type Key%20Structure :default "None"))
  ;[1 1 1] CAMERA FADE
  (:Pressed
    (CameraFades|StartCameraFade :self (Game|GetPlayerCameraManager 0) :ToAlpha 1.0 :Duration 1.0 :bHoldWhenFinished true)
    (Utilities|FlowControl|Delay 2.0)
    (CallFunction|ShowSittingAvatars)
    (bind _outactors (Actor|GetAllActorsOfClass "/Game/Assets/ThirdPerson/Blueprints/BP_ThirdPersonCharacter.BP_ThirdPersonCharacter_C"))
    (for _array_element _outactors
      (Rendering|SetVisibility (Variables|/Script/Engine.Character|GetMesh _array_element) false false)
      (CameraFades|StartCameraFade :self (Game|GetPlayerCameraManager 0) :FromAlpha 1.0 :Duration 1.0 :bHoldWhenFinished true)
      (Input|DisableInput (Variables|Default|GetThirdPersonBP_Ref) (Game|GetPlayerController 0)))))

(event Input|KeyboardEvents|2
  (params (Key :type Key%20Structure :default "None"))
  (:Pressed
    (bind _returnvalue (Actor|GetActorOfClass "/Game/VirtualWorld/InGameBrowser/Blueprints/BP_WebBrowser.BP_WebBrowser_C"))
    (Utilities|IsValid _returnvalue
      (:Is%20Valid
        (Actor|DestroyActor _returnvalue)
        (Game|SpawnActorfromClass "/Game/VirtualWorld/InGameBrowser/Blueprints/BP_Listings.BP_Listings_C" (Math|Transform|MakeTransform "-295.000000,4452.000000,380.000000" "0, 0, 0" "1.000000,1.000000,1.000000") "Undefined" 0 0))
      (:Is%20Not%20Valid
        (Game|SpawnActorfromClass "/Game/VirtualWorld/InGameBrowser/Blueprints/BP_Listings.BP_Listings_C" (Math|Transform|MakeTransform "-295.000000,4452.000000,380.000000" "0, 0, 0" "1.000000,1.000000,1.000000") "Undefined" 0 0)))))

(event Input|KeyboardEvents|3
  (params (Key :type Key%20Structure :default "None"))
  (:Pressed
    (bind _returnvalue (Actor|GetActorOfClass "/Game/VirtualWorld/InGameBrowser/Blueprints/BP_Listings.BP_Listings_C"))
    (Utilities|IsValid _returnvalue
      (:Is%20Valid
        (Actor|DestroyActor _returnvalue)
        (Game|SpawnActorfromClass "/Game/VirtualWorld/InGameBrowser/Blueprints/BP_WebBrowser.BP_WebBrowser_C" (Math|Transform|MakeTransform "-295.000000,4452.000000,380.000000" "0, 0, 0" "1.000000,1.000000,1.000000") "Undefined" 0 0))
      (:Is%20Not%20Valid
        (Game|SpawnActorfromClass "/Game/VirtualWorld/InGameBrowser/Blueprints/BP_WebBrowser.BP_WebBrowser_C" (Math|Transform|MakeTransform "-295.000000,4452.000000,380.000000" "0, 0, 0" "1.000000,1.000000,1.000000") "Undefined" 0 0)))))

(fn ConstructionScript)